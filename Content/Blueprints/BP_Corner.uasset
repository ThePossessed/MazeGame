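; BP_Corner is a paintable mesh actor that the player draws on while holding the left mouse button.
; BeginPlay creates a cleared render target and feeds it into a dynamic wall material on the mesh.
; Each Tick traces from an offset camera point against the mesh, converts the hit to UVs, and draws a colored polygon dot onto that target.
; A brush material instance is created but unused, and the canvas draw is never explicitly ended.
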(event EventBeginPlay
  ;[1 1 1] Create dynamic material instances
  (Utilities|FlowControl|Sequence
    (:then_0
      (bind _returnvalue (Rendering|CreateRenderTarget2D 1024 1024 "RTF_RGBA16f"))
      (bind _output_get (Variables|Default|SetRenderTarget _returnvalue))
      (Rendering|ClearRenderTarget2D _output_get))
    (:then_1
      (bind _returnvalue_2 (Rendering|Material|CreateDynamicMaterialInstance "/Game/Meshes/Materials/WallMat.WallMat" "None" :!class /Script/Engine.KismetMaterialLibrary))
      (Rendering|Material|SetTextureParameterValue _returnvalue_2 "RenderTarget" (Variables|Default|GetRenderTarget))
      (Rendering|Material|SetMaterial (Variables|Default|GetStaticMesh) 0 _returnvalue_2))
    (:then_2
      (bind _returnvalue_3 (Rendering|Material|CreateDynamicMaterialInstance "/Game/Meshes/Materials/BrushMat.BrushMat" "None" :!class /Script/Engine.KismetMaterialLibrary))
      (Variables|Default|SetBrushMaterial _returnvalue_3))))

(event EventTick
  (params (DeltaSeconds :type Float%20%28single-precision%29))
  (bind _returnvalue (Game|GetPlayerCameraManager 0))
  (bind _returnvalue_2 (Camera|GetCameraRotation _returnvalue))
  (bind _transformcomponent (Variables|/Script/Engine.PlayerCameraManager|GetTransformComponent _returnvalue))
  (bind _returnvalue_3 (Math|Vector|GetRightVector _returnvalue_2))
  (bind _returnvalue_4 (Transformation|GetWorldLocation _transformcomponent))
  (bind _returnvalue_5 (Math|Vector|GetUpVector _returnvalue_2))
  (bind _returnvalue_6 (* _returnvalue_3 5e+01))
  (bind _returnvalue_7 (* _returnvalue_5 75.0))
  (bind _returnvalue_8 (+ _returnvalue_6 _returnvalue_4))
  (bind _returnvalue_9 (+ _returnvalue_7 _returnvalue_8))
  ;[1 1 1] Draw
  (bind (_hitlocation _hitnormal _bonename _outhit _returnvalue_10) (Collision|LineTraceComponent (Variables|Default|GetStaticMesh) _returnvalue_9 (+ _returnvalue_9 (* (Math|Vector|GetForwardVector _transformcomponent) 4.5e+02)) true false false))
  (if _returnvalue_10
    (if (Game|Player|IsInputKeyDown (Game|GetPlayerController 0) "LeftMouseButton")
      (bind (_canvas _size) (Rendering|BeginDrawCanvastoRenderTarget (Variables|Default|GetRenderTarget)))
      (Class|Canvas|DrawPolygon _canvas 0 (* (.UV (Class|GameplayStatics|FindCollisionUV _outhit)) _size) "(X=10.000000,Y=10.000000)" 32 "(R=1.000000,G=0.008445,B=0.068168,A=1.000000)"))))

(fn ConstructionScript)