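; BP_Wall is a wall the player paints on by looking at it and holding E.
; BeginPlay clears the render target, then each Tick traces against the wall's static mesh along the camera's forward vector.
; While E is held, a hit draws a debug sphere and converts its collision UV to canvas coordinates for a small polygon dot.
; The canvas draw has no matching EndDrawCanvasToRenderTarget call.
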(event EventBeginPlay
  (bind _rendertarget (Variables|Default|GetRenderTarget))
  (Rendering|ClearRenderTarget2D _rendertarget (Variables|/Script/Engine.TextureRenderTarget2D|GetClearColor _rendertarget)))

(event EventTick
  (params (DeltaSeconds :type Float%20%28single-precision%29))
  (bind _returnvalue (Game|GetPlayerCameraManager 0))
  (bind _transformcomponent (Variables|/Script/Engine.PlayerCameraManager|GetTransformComponent _returnvalue))
  (bind _returnvalue_2 (Transformation|GetWorldLocation _transformcomponent))
  (bind (_hitlocation _hitnormal _bonename _outhit _returnvalue_3) (Collision|LineTraceComponent (Variables|Default|GetStaticMesh) _returnvalue_2 (+ _returnvalue_2 (* (Math|Vector|GetForwardVector _transformcomponent) 1e+05)) true false false))
  (if _returnvalue_3
    (if (Game|Player|IsInputKeyDown (Game|GetPlayerController 0) "E")
      (Rendering|Debug|DrawDebugSphere _hitlocation 1e+02 12 "(R=1.000000,G=1.000000,B=1.000000,A=1.000000)" 0.0)
      (bind (_canvas _size) (Rendering|BeginDrawCanvastoRenderTarget (Variables|Default|GetRenderTarget)))
      (Class|Canvas|DrawPolygon _canvas 0 (* (.UV (Class|GameplayStatics|FindCollisionUV _outhit)) _size) "(X=1.000000,Y=1.000000)" 16 "(R=1.000000,G=1.000000,B=1.000000,A=1.000000)"))))

(fn ConstructionScript)